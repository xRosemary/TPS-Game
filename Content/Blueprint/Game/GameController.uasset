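; Player controller that handles the client's opening flow from an interlude screen to the login menu.
; On BeginPlay, when not running as server, it creates the interlude widget, adds it to the viewport and shows the mouse cursor.
; The first key press sets a one-shot skip flag and, if the interlude is valid, swaps it for the main login widget.
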(event EventBeginPlay
  (if (not (Networking|IsServer))
    (bind _returnvalue (UserInterface|CreateWidget "/Game/Blueprint/UI/Interlude/UI_Interlude_BP.UI_Interlude_BP_C"))
    (bind _output_get (Variables|Default|SetInterlude _returnvalue))
    (UserInterface|Viewport|AddtoViewport _output_get 0)
    (Variables|Default|SetbShowMouseCursor true)))

(event Input|KeyboardEvents|AnyKey
  (params (Key :type Key%20Structure :default "None"))
  (bind _interlude (Variables|Default|GetInterlude))
  (:Pressed
    (if (not (Variables|Default|GetbSkipped))
      (Variables|Default|SetbSkipped true)
      (Utilities|IsValid _interlude
        (:Is%20Valid
          (Widget|RemovefromParent _interlude)
          (bind _returnvalue (UserInterface|CreateWidget "/Game/Blueprint/UI/Login/UI_LoginMain_BP.UI_LoginMain_BP_C"))
          (bind _output_get (Variables|Default|SetLoginMenu _returnvalue))
          (UserInterface|Viewport|AddtoViewport _output_get 0))))))

(fn ConstructionScript)