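; PlayGameController is a player controller that handles spawning and possessing the player's character in play.
; StartSpawnCharacter waits briefly, then asks PlayGameMode to spawn for this controller through RequestSpawn.
; SpawnPlayerCharacter spawns the given class at a transform, possesses it, then calls ClientHideMouse to switch to game-only input and hide the cursor.
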(event Custom|SpawnPlayerCharacter
  (params (Class :type Character%20Base%20Class%20Reference) (SpawnTransform :type Transform))
  (bind _returnvalue (Game|SpawnActorfromClass Class SpawnTransform "Undefined" 0 0))
  (Pawn|Possess _returnvalue)
  (CallFunction|ClientHideMouse))

(event Custom|StartSpawnCharacter
  (Utilities|FlowControl|Delay 1.0)
  (bind _asplay_game_mode (Utilities|Casting|CastToPlayGameMode (Game|GetGameMode)))
  (Default|RequestSpawn _asplay_game_mode self))

(event Custom|ClientHideMouse
  (Input|SetInputModeGameOnly self)
  (Variables|Default|SetbShowMouseCursor false))

(fn ConstructionScript)